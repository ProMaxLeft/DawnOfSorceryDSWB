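; BP_HPotion is a health potion pickup that heals the player character on overlap.
; When the Sphere overlaps a BP actor below its HealthLimit, it adds a fixed amount of Health, clamped to that limit, then destroys itself.
; At full health the potion stays in the world.
; BeginPlay casts the player pawn to BP but does nothing with the result.
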(event `self.ReceiveBeginPlay`
  (cast `/Game/Characters/Char/BP` (`GameplayStatics.GetPlayerPawn` 0)))

(event `self.Sphere.OnComponentBeginOverlap`
  (params (OverlappedComponent :type "PrimitiveComponent Object Reference") (OtherActor :type "Actor Object Reference") (OtherComp :type "PrimitiveComponent Object Reference") (OtherBodyIndex :type Integer) (bFromSweep :type Boolean) (SweepResult :type "HitResult Structure (by ref)"))
  (bind _asbp (cast `/Game/Characters/Char/BP` OtherActor))
  (bind _healthlimit (`/Game/Characters/Char/BP.HealthLimit` _asbp))
  (if (< (`/Game/Characters/Char/BP.Health` _asbp) _healthlimit)
    (set `/Game/Characters/Char/BP.Health` (`KismetMathLibrary.FClamp` (+ (`/Game/Characters/Char/BP.Health` _asbp) 30.0) 0.0 _healthlimit) _asbp)
    (`self.K2_DestroyActor`)))

(fn `UserConstructionScript`)