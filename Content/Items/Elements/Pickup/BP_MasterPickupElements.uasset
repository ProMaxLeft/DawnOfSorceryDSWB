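; BP_MasterPickupElements is an element pickup actor that the player collects by interacting while inside its collision area.
; Overlap start binds PickupElement to the character's interact event and shows its pickup HUD; overlap end reverses both.
; PickupElement asks the player character, cached on BeginPlay, to spawn the configured element at its socket, then destroys the pickup if that succeeds.
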(event `self.pickupcollision.OnComponentBeginOverlap`
  (params (OverlappedComponent :type "PrimitiveComponent Object Reference") (OtherActor :type "Actor Object Reference") (OtherComp :type "PrimitiveComponent Object Reference") (OtherBodyIndex :type Integer) (bFromSweep :type Boolean) (SweepResult :type "HitResult Structure (by ref)"))
  (bind _asbp (cast `/Game/Characters/Char/BP` OtherActor))
  (add `/Game/Characters/Char/BP.InteractObjects` _asbp (delegate `PickupElement`))
  (bind _elementpickuphud (`/Game/Characters/Char/BP.ElementPickupHud` _asbp))
  (if (not (`Widget.IsInViewport` _elementpickuphud))
    (`UserWidget.AddToViewport` _elementpickuphud 0)))

(event `self.pickupcollision.OnComponentEndOverlap`
  (params (OverlappedComponent :type "PrimitiveComponent Object Reference") (OtherActor :type "Actor Object Reference") (OtherComp :type "PrimitiveComponent Object Reference") (OtherBodyIndex :type Integer))
  (bind _asbp (cast `/Game/Characters/Char/BP` OtherActor))
  (remove `/Game/Characters/Char/BP.InteractObjects` _asbp (delegate `PickupElement`))
  (`Widget.RemoveFromParent` (`/Game/Characters/Char/BP.ElementPickupHud` _asbp)))

(event `PickupElement`
  (bind _success (`/Game/Characters/Char/BP.SpawnElements` (`self.CharacterRef`) (`self.Element`) (`self.ElementSocket`)))
  (if _success
    (`self.K2_DestroyActor`)))

(event `self.ReceiveBeginPlay`
  (bind _asbp (cast `/Game/Characters/Char/BP` (`GameplayStatics.GetPlayerPawn` 0)))
  (set `self.CharacterRef` _asbp))

(fn `UserConstructionScript`)