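; BP_Red is a player-controlled Character with camera look, movement, jumping and a simple health and death flow.
; It registers the default Enhanced Input mapping context on BeginPlay, then drives controller yaw and pitch, movement relative to control rotation, and jumping from input actions.
; A hardcoded 1 key subtracts clamped health and, at zero, shows the mouse cursor and a death-to-menu widget.
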(event `self.ReceiveBeginPlay`
  ; движ
  (bind _asplayer_controller (cast `PlayerController` (`self.GetController`)))
  (bind _returnvalue (pcsubsystem `EnhancedInputLocalPlayerSubsystem` _asplayer_controller))
  (`/Engine/EditorBlueprintResources/StandardMacros.IsValid` _returnvalue
    (:`Is Valid`
      (`EnhancedInputSubsystemInterface.AddMappingContext` _returnvalue "/Game/Characters/IMC_Default.IMC_Default" 0 (struct)))))

(event `EnhancedInput|/Game/Characters/Input/IA_Look`
  (params (ActionValue :type "Vector2D Structure") (ElapsedSeconds :type "Float (double-precision)") (TriggeredSeconds :type "Float (double-precision)") (InputAction :type "InputAction Object Reference" :default "/Game/Characters/Input/IA_Look.IA_Look"))
  ; камера
  (:`Triggered`
    ;; лева-права
    (`self.AddControllerYawInput` ActionValue_X)
    ;; верх-низ
    (`self.AddControllerPitchInput` ActionValue_Y)))

(event `EnhancedInput|/Game/Characters/Input/IA_Move`
  (params (ActionValue :type "Vector2D Structure") (ElapsedSeconds :type "Float (double-precision)") (TriggeredSeconds :type "Float (double-precision)") (InputAction :type "InputAction Object Reference" :default "/Game/Characters/Input/IA_Move.IA_Move"))
  (bind (_returnvalue_roll _returnvalue_pitch _returnvalue_yaw) (`KismetMathLibrary.BreakRotator` (`self.GetControlRotation`)))
  (bind (_returnvalue_roll_2 _returnvalue_pitch_2 _returnvalue_yaw_2) (`KismetMathLibrary.BreakRotator` (`self.GetControlRotation`)))
  ; Движ конкретный
  (:`Triggered`
    ;; лева-права движ
    (`self.AddMovementInput` (`KismetMathLibrary.GetRightVector` (`KismetMathLibrary.MakeRotator` _returnvalue_roll 0.0 _returnvalue_yaw)) ActionValue_X)
    ;; перед-зад
    (`self.AddMovementInput` (`KismetMathLibrary.GetForwardVector` (`KismetMathLibrary.MakeRotator` 0.0 0.0 _returnvalue_yaw_2)) ActionValue_Y)))

(event `EnhancedInput|/Game/Characters/Input/IA_Jump`
  (params (ActionValue :type Boolean) (ElapsedSeconds :type "Float (double-precision)") (TriggeredSeconds :type "Float (double-precision)") (InputAction :type "InputAction Object Reference" :default "/Game/Characters/Input/IA_Jump.IA_Jump"))
  ; Прыжок
  (:`Triggered`
    (`self.Jump`))
  (:`Completed`
    (`self.StopJumping`)))

(event `Key|One`
  (params (Key :type "Key Structure"))
  (:`Pressed`
    (set `self.Health` (`KismetMathLibrary.FClamp` (- (`self.Health`) 20.0) 0.0 (`self.HealthLimit`)))
    (if (== (`self.Health`) 0.0)
      (set `PlayerController.bShowMouseCursor` true (`GameplayStatics.GetPlayerController` 0))
      (bind _returnvalue (`|CreateWidget` "/Game/Characters/Char/UI/Death/DeathWidgetToMenu.DeathWidgetToMenu_C"))
      (`UserWidget.AddToViewport` _returnvalue 0))))

(fn `UserConstructionScript`)