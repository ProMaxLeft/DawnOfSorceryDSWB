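; BP_ManaPotion2 is a mana potion pickup that adds one potion to the player character's count.
; On BeginPlay it caches the player pawn as a BP character reference.
; When a BP character overlaps its sphere and the cached player is below the potion cap, it increments the count, updates the character widget's HP element and destroys itself.
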(event `self.ReceiveBeginPlay`
  (bind _asbp (cast `/Game/Characters/Char/BP` (`GameplayStatics.GetPlayerPawn` 0)))
  (set `self.CharRef` _asbp))

(event `self.Sphere.OnComponentBeginOverlap`
  (params (OverlappedComponent :type "PrimitiveComponent Object Reference") (OtherActor :type "Actor Object Reference") (OtherComp :type "PrimitiveComponent Object Reference") (OtherBodyIndex :type Integer) (bFromSweep :type Boolean) (SweepResult :type "HitResult Structure (by ref)"))
  (bind _charref (`self.CharRef`))
  (bind _charref_2 (`self.CharRef`))
  (cast `/Game/Characters/Char/BP` OtherActor)
  (if (< (`/Game/Characters/Char/BP.ManaPotion` _charref) (`/Game/Characters/Char/BP.MaxManaPotion` _charref))
    (bind _output_get (set `/Game/Characters/Char/BP.ManaPotion` (+ (`/Game/Characters/Char/BP.ManaPotion` _charref_2) 1) _charref_2))
    (`/Game/Characters/Char/UI/HPHud/HP.UpdateHPSystem` (`/Game/Characters/Char/CharWidget.HP` (`/Game/Characters/Char/BP.CharWidget` (`self.CharRef`))) 0.0 0.0 "NewEnumerator3" _output_get)
    (`self.K2_DestroyActor`)))

(fn `UserConstructionScript`)