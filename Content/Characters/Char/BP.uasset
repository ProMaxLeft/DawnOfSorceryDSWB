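; Player character with Enhanced Input movement, health, regenerating mana and elemental attacks.
; Number keys drain stats or grant Water and Fire, which combine into Steam; LMB repeats mana-costing fireballs, Shift+LMB spawns Fire or Steam circles.
; Zero health shows a death widget and respawns via the Football game mode, but AnyDamage never triggers that check.
; SpawnElements swaps element child actors between hip and back sockets, uncalled here.
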(event `self.ReceiveBeginPlay`
  (bind _returnvalue (`GameplayStatics.GetPlayerController` 0))
  ; движ
  (`|ExecutionSequence`
    (:`then_0`
      (bind _asplayer_controller (cast `PlayerController` (`self.GetController`)))
      (bind _returnvalue_2 (pcsubsystem `EnhancedInputLocalPlayerSubsystem` _asplayer_controller))
      (`/Engine/EditorBlueprintResources/StandardMacros.IsValid` _returnvalue_2
        (:`Is Valid`
          (`EnhancedInputSubsystemInterface.AddMappingContext` _returnvalue_2 "/Game/Characters/IMC_Default.IMC_Default" 0 (struct)))))
    (:`then_1`
      ; Для виджетов в целом
      (`self.CreateWidgets`))
    (:`then_2`
      ; Смерть и условия для респавна
      (if (== (`self.Health`) 0.0) :!label _label
        (`self.K2_DestroyActor`)
        (set `PlayerController.bShowMouseCursor` true _returnvalue)
        (set `PlayerController.bEnableMotionControls` true _returnvalue)
        (bind _returnvalue_3 (`|CreateWidget` "/Game/Characters/Char/UI/Death/DeathWidgetToMenu.DeathWidgetToMenu_C"))
        (`UserWidget.AddToViewport` _returnvalue_3 0)
        (`KismetSystemLibrary.Delay` 5.0)
        (set `PlayerController.bShowMouseCursor` false (`GameplayStatics.GetPlayerController` 0))
        (`WidgetLayoutLibrary.RemoveAllWidgets`)
        (bind _asfootball (cast `/Game/Characters/football_ball/Football` (`GameplayStatics.GetGameMode`)))
        (`/Game/Characters/football_ball/Football.Respawn` _asfootball (`self.GetInstigatorController`))))))

(event `EnhancedInput|/Game/Characters/Input/IA_Look`
  (params (ActionValue :type "Vector2D Structure") (ElapsedSeconds :type "Float (double-precision)") (TriggeredSeconds :type "Float (double-precision)") (InputAction :type "InputAction Object Reference" :default "/Game/Characters/Input/IA_Look.IA_Look"))
  ; камера
  (:`Triggered`
    ;; лева-права
    (`self.AddControllerYawInput` ActionValue_X)
    ;; верх-низ
    (`self.AddControllerPitchInput` ActionValue_Y)))

(event `EnhancedInput|/Game/Characters/Input/IA_Move`
  (params (ActionValue :type "Vector2D Structure") (ElapsedSeconds :type "Float (double-precision)") (TriggeredSeconds :type "Float (double-precision)") (InputAction :type "InputAction Object Reference" :default "/Game/Characters/Input/IA_Move.IA_Move"))
  (bind (_returnvalue_roll _returnvalue_pitch _returnvalue_yaw) (`KismetMathLibrary.BreakRotator` (`self.GetControlRotation`)))
  (bind (_returnvalue_roll_2 _returnvalue_pitch_2 _returnvalue_yaw_2) (`KismetMathLibrary.BreakRotator` (`self.GetControlRotation`)))
  ; Движ конкретный
  (:`Triggered`
    ;; лева-права движ
    (`self.AddMovementInput` (`KismetMathLibrary.GetRightVector` (`KismetMathLibrary.MakeRotator` _returnvalue_roll 0.0 _returnvalue_yaw)) ActionValue_X)
    ;; перед-зад
    (`self.AddMovementInput` (`KismetMathLibrary.GetForwardVector` (`KismetMathLibrary.MakeRotator` 0.0 0.0 _returnvalue_yaw_2)) ActionValue_Y)))

(event `EnhancedInput|/Game/Characters/Input/IA_Jump`
  (params (ActionValue :type Boolean) (ElapsedSeconds :type "Float (double-precision)") (TriggeredSeconds :type "Float (double-precision)") (InputAction :type "InputAction Object Reference" :default "/Game/Characters/Input/IA_Jump.IA_Jump"))
  ; Прыжок
  (:`Triggered`
    (`self.Jump`))
  (:`Completed`
    (`self.StopJumping`)))

(event `self.ReceiveAnyDamage`
  (params (Damage :type "Float (single-precision)") (DamageType :type "DamageType Object Reference") (InstigatedBy :type "Controller Object Reference") (DamageCauser :type "Actor Object Reference"))
  (bind _output_get (set `self.Health` (- (`self.Health`) Damage)))
  (`KismetSystemLibrary.PrintString` (`KismetStringLibrary.Conv_DoubleToString` _output_get)))

(event `Key|One`
  (params (Key :type "Key Structure"))
  ; Здоровье
  (:`Pressed`
    (set `self.Health` (`KismetMathLibrary.FClamp` (- (`self.Health`) 20.0) 0.0 (`self.HealthLimit`)))
    (goto _label)))

(event `Key|Two`
  (params (Key :type "Key Structure"))
  ; Мана
  (:`Pressed`
    (set `self.Mana` (`KismetMathLibrary.FClamp` (- (`self.Mana`) 20.0) 0.0 (`self.ManaLimit`)))))

(event `self.ReceiveTick`
  (params (DeltaSeconds :type "Float (single-precision)"))
  ; Восстановление маны
  (`KismetSystemLibrary.Delay` 1.0)
  (set `self.Mana` (`KismetMathLibrary.FClamp` (+ (`self.Mana`) 1.0) 0.0 (`self.ManaLimit`))))

(event `Key|Shift+LeftMouseButton`
  (params (Key :type "Key Structure"))
  (:`Pressed`
    (if (`self.Fire?`)
      (`ActorComponent.K2_DestroyComponent` (`self.ElementFire`))
      (`self.FireAroundSelf`)
      (set `self.Fire?` false)
      (elif (`self.Steam?`)
        (`self.SteamAroundSelf`)))))

(event `FireAroundSelf`
  (`|SpawnActorFromClass` "/Game/Items/Elements/ElementsOnInterract/Fire/Around/FireCircle.FireCircle_C" (`KismetMathLibrary.Conv_VectorToTransform` (`self.K2_GetActorLocation`)) "Undefined" "MultiplyWithRoot" null null))

(event `SteamAroundSelf`
  (`|SpawnActorFromClass` "/Game/Items/Elements/ElementsOnInterract/CombinationElement/Steam/SteamCircle.SteamCircle_C" (`KismetMathLibrary.Conv_VectorToTransform` (`self.K2_GetActorLocation`)) "Undefined" "MultiplyWithRoot" null null))

(event `Key|Four`
  (params (Key :type "Key Structure"))
  (:`Pressed`
    (set `self.Water?` true)
    (if (and (`self.Fire?`) (`self.Water?`)) :!label _label
      (set `self.Water?` false)
      (set `self.Fire?` false)
      (`ActorComponent.K2_DestroyComponent` (`self.ElementFire`))
      (set `self.Steam?` true))))

(event `Key|Five`
  (params (Key :type "Key Structure"))
  (:`Pressed`
    (set `self.Fire?` true)
    (bind _returnvalue (`|AddComponentByClass` "/Game/Items/Elements/ElementsOnInterract/Fire/ElementtFire.ElementtFire_C" false (`KismetMathLibrary.Conv_VectorToTransform` (+ (`self.K2_GetActorLocation` (`GameplayStatics.GetPlayerPawn` 0)) (0.0 0.0 0.0)))))
    (set `self.ElementFire` _returnvalue)
    (goto _label)))

(event `InputAction|LMB`
  (params (Key :type "Key Structure"))
  (bind _returnvalue (`GameplayStatics.GetPlayerCameraManager` 0))
  (:`Pressed`
    (set `self.LmbIsTrue?` true)
    (if (`self.Fire?`)
      (set `self.ManaYES?` (>= (`self.Mana`) 10.0) :!label _label_2)
      (set `self.IsFiring?` true)
      (if (`self.ManaYES?`)
        (set `self.Mana` (- (`self.Mana`) 10.0))
        (bind _outactors (`GameplayStatics.GetAllActorsOfClass` "BP_C"))
        (`KismetSystemLibrary.LineTraceSingle` (`self.K2_GetActorLocation` (`GameplayStatics.GetPlayerPawn` 0)) (+ (`PlayerCameraManager.GetCameraLocation` _returnvalue) (* (`self.GetActorForwardVector` _returnvalue) (`self.Range`))) "TraceTypeQuery1" false _outactors "ForDuration")
        (`|SpawnActorFromClass` "/Game/Items/Elements/ElementsOnInterract/Fire/LMB/FireBallGoGo.FireBallGoGo_C" (`KismetMathLibrary.MakeTransform` (+ (`self.K2_GetActorLocation`) (150.0 150.0 150.0)) (`SceneComponent.K2_GetComponentRotation` (`self.Camera`))) "Undefined" "MultiplyWithRoot" null null)
        (if (`self.IsFiring?`)
          (`KismetSystemLibrary.Delay` 0.2)
          (if (`self.IsFiring?`)
            (goto _label_2)
            (else
              (set `self.Fire?` false)
              (`ActorComponent.K2_DestroyComponent` (`self.ElementFire`))))))))
  (:`Released`
    (set `self.LmbIsTrue?` false)
    (set `self.IsFiring?` false)))

(fn `CreateWidgets`
  (bind _returnvalue (`|CreateWidget` "/Game/Items/Elements/UI/WB_ElementPickup.WB_ElementPickup_C"))
  (set `self.ElementPickupHud` _returnvalue))

(fn `SpawnElements`
  (params (Element :type "/Game/Items/Elements/ElementsOnInterract/BP_MasterElements Class Reference") (ElementSocket :type "/Game/Items/Elements/Enum/ElementSocketEnum Enum" :default "NewEnumerator0"))
  (returns (success :type Boolean))
  (locals (NewLocalVar :type "/Game/Items/Elements/Enum/ElementSocketEnum Enum" :default "NewEnumerator0"))
  (bind _backelement (`self.BackElement`))
  (bind _hipelement (`self.HipElement`))
  (set `self.LocalElement` Element)
  (set `self.LocalElementSocket` ElementSocket)
  (switch `/Game/Items/Elements/Enum/HasElementEnum` (`self.HasElement`)
    (:`NewEnumerator0`
      (if (not (`|EnumEquality` (`self.LocalElementSocket`) (`self.CurrentElementSocket`)))
        (switch `/Game/Items/Elements/Enum/ElementSocketEnum` (`self.CurrentElementSocket`)
          (:`NewEnumerator0`
            (`SceneComponent.K2_AttachToComponent` (`self.HipElement`) (`self.HipElementSocket`) "None" "SnapToTarget" "SnapToTarget" "SnapToTarget" true)
            (set `self.HolsterElement` (`self.CurrentElement`))
            (set `self.HolsterElementSocket` (`self.CurrentElementSocket`))
            (`ChildActorComponent.SetChildActorClass` _backelement (`self.LocalElement`) :!label _label)
            (bind _asbp_master_elements (cast `/Game/Items/Elements/ElementsOnInterract/BP_MasterElements` (`ChildActorComponent.ChildActor` _backelement)))
            (set `self.CurrentElement` _asbp_master_elements)
            (set `self.CurrentElementSocket` "NewEnumerator1")
            (`SceneComponent.K2_AttachToComponent` (`self.BackElement`) null "None" "SnapToTarget" "SnapToTarget" "SnapToTarget" true))
          (:`NewEnumerator1`
            (`SceneComponent.K2_AttachToComponent` (`self.BackElement`) (`self.BackElementSocket`) "None" "SnapToTarget" "SnapToTarget" "SnapToTarget" true)
            (set `self.HolsterElement` (`self.CurrentElement`))
            (set `self.HolsterElementSocket` (`self.CurrentElementSocket`))
            (`ChildActorComponent.SetChildActorClass` _hipelement (`self.LocalElement`) :!label _label_2)
            (bind _asbp_master_elements_2 (cast `/Game/Items/Elements/ElementsOnInterract/BP_MasterElements` (`ChildActorComponent.ChildActor` _hipelement)))
            (set `self.CurrentElement` _asbp_master_elements_2)
            (set `self.CurrentElementSocket` "NewEnumerator0")
            (`SceneComponent.K2_AttachToComponent` (`self.HipElement`) null "None" "SnapToTarget" "SnapToTarget" "SnapToTarget" true)))
        (set `self.HasElement` "NewEnumerator0")
        (return true)))
    (:`NewEnumerator1`
      (switch `/Game/Items/Elements/Enum/ElementSocketEnum` (`self.LocalElementSocket`)
        (:`NewEnumerator0`
          (goto _label_2))
        (:`NewEnumerator1`
          (goto _label))))))

(fn `UserConstructionScript`)